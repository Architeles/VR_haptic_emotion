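; Controller Blueprint that drives a referenced Niagara particle system from Leap Motion hand gestures.
; On BeginPlay it sets the User noise strength, particle rate and drag parameters on the NiagraRef component to starting values.
; Grabbing lowers noise and raises rate and drag, while releasing restores noise and drag but pushes the particle rate far above its starting value.
; The pinch event is empty.
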(event `self.ReceiveBeginPlay`
  (bind _niagaracomponent (`NiagaraActor.NiagaraComponent` (`self.niagraRef`)))
  (`FXSystemComponent.SetFloatParameter` _niagaracomponent "User.noiseStrength" 20000.0)
  (`FXSystemComponent.SetFloatParameter` _niagaracomponent "User.particleRate" 100.0)
  (`FXSystemComponent.SetFloatParameter` _niagaracomponent "User.dragStrength" 10.0))

(event `self.Leap.OnHandGrabbed`
  (params (Hand :type "LeapHandData Structure (by ref)"))
  (bind _niagaracomponent (`NiagaraActor.NiagaraComponent` (`self.niagraRef`)))
  (`FXSystemComponent.SetFloatParameter` _niagaracomponent "User.noiseStrength" 5000.0)
  (`FXSystemComponent.SetFloatParameter` _niagaracomponent "User.particleRate" 1000.0)
  (`FXSystemComponent.SetFloatParameter` _niagaracomponent "User.dragStrength" 20.0))

(event `self.Leap.OnHandReleased`
  (params (Hand :type "LeapHandData Structure (by ref)"))
  (bind _niagaracomponent (`NiagaraActor.NiagaraComponent` (`self.niagraRef`)))
  (`FXSystemComponent.SetFloatParameter` _niagaracomponent "User.noiseStrength" 20000.0)
  (`FXSystemComponent.SetFloatParameter` _niagaracomponent "User.particleRate" 10000.0)
  (`FXSystemComponent.SetFloatParameter` _niagaracomponent "User.dragStrength" 10.0))

(event `self.Leap.OnHandPinched`
  (params (Hand :type "LeapHandData Structure (by ref)")))

(fn `UserConstructionScript`)