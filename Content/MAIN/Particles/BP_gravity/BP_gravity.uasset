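; BP_gravity is a gravity point that pulls every BP_gravity_objects cube toward a center by adding velocity each tick.
; The center is its own CubeG when IsLaHp or IsCenterOfGravityACube is set, otherwise the right thumb-end capsule of an IEUICollisionLowPolyHand, with a stronger pull.
; In cube-centered mode, a delayed distance check spawns another tagged cube near GI_Master's spawn location when all cubes are beyond a threshold.
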(event `self.ReceiveTick`
  (params (DeltaSeconds :type "Float (single-precision)"))
  (if (`self.is_la_hp?`)
    (bind _outactors (`GameplayStatics.GetAllActorsOfClass` "/Game/Lisa/Particles/BP_gravity/BP_gravity_objects.BP_gravity_objects_C" :!label _label))
    (for _array_element _outactors
      (`PrimitiveComponent.SetPhysicsLinearVelocity` (`/Game/Lisa/Particles/BP_gravity/BP_gravity_objects.Cube` _array_element) (* (`KismetMathLibrary.GetForwardVector` (`KismetMathLibrary.FindLookAtRotation` (`SceneComponent.K2_GetComponentLocation` (`/Game/Lisa/Particles/BP_gravity/BP_gravity_objects.Cube` _array_element)) (`SceneComponent.K2_GetComponentLocation` (`self.Cube_g`)))) 0.1) true "None")
      (`KismetSystemLibrary.Delay` 2.0)
      (`self.getDistance`))
    (elif (`self.isCenterOfGravityACube?`)
      (goto _label)
      (else
        (bind _outactors_2 (`GameplayStatics.GetAllActorsOfClass` "/UltraleapTracking/InteractionEngine/Pawn/IEUICollisionLowPolyHand.IEUICollisionLowPolyHand_C"))
        (set `self.Capsule R Thumb End` (`/UltraleapTracking/InteractionEngine/Pawn/IEUICollisionLowPolyHand.Capsule_R_thumb_end` (`|GetArrayItem` _outactors_2)))
        (bind _outactors_3 (`GameplayStatics.GetAllActorsOfClass` "/Game/Lisa/Particles/BP_gravity/BP_gravity_objects.BP_gravity_objects_C"))
        (for _array_element_2 _outactors_3
          (`PrimitiveComponent.SetPhysicsLinearVelocity` (`/Game/Lisa/Particles/BP_gravity/BP_gravity_objects.Cube` _array_element_2) (* (`KismetMathLibrary.GetForwardVector` (`KismetMathLibrary.FindLookAtRotation` (`SceneComponent.K2_GetComponentLocation` (`/Game/Lisa/Particles/BP_gravity/BP_gravity_objects.Cube` _array_element_2)) (`SceneComponent.K2_GetComponentLocation` (`self.Capsule R Thumb End`)))) 1.0) true "None"))))))

(fn `getDistance`
  (`KismetArrayLibrary.Array_Clear` (`self.distanceArray`))
  (bind _outactors (`GameplayStatics.GetAllActorsOfClass` "/Game/Lisa/Particles/BP_gravity/BP_gravity_objects.BP_gravity_objects_C"))
  (for _array_element _outactors
    (`KismetArrayLibrary.Array_Add` (`self.distanceArray`) (`KismetMathLibrary.VSize` (- (`SceneComponent.K2_GetComponentLocation` (`self.Cube_g`)) (`SceneComponent.K2_GetComponentLocation` (`/Game/Lisa/Particles/BP_gravity/BP_gravity_objects.Cube` _array_element))))))
  (if (> (`.MinValue` (`VictoryBPFunctionLibrary.MinOfFloatArray` (`self.distanceArray`))) 50.0)
    (`self.spawnCube`)))

(fn `spawnCube`
  (bind _asgi_master (cast `/Game/Lisa/GI_Master` (`GameplayStatics.GetGameInstance`)))
  (bind (_gravity_point_spawn_loc_x _gravity_point_spawn_loc_y _gravity_point_spawn_loc_z) (`KismetMathLibrary.BreakVector` (`/Game/Lisa/GI_Master.Gravity_point_spawn_loc` _asgi_master)))
  (bind _returnvalue (`|SpawnActorFromClass` "/Game/Lisa/Particles/BP_gravity/BP_gravity_objects.BP_gravity_objects_C" (`KismetMathLibrary.MakeTransform` (`KismetMathLibrary.MakeVector` (+ _gravity_point_spawn_loc_x (`KismetMathLibrary.RandomFloatInRange` -30.0 30.0)) (+ _gravity_point_spawn_loc_y (`KismetMathLibrary.RandomFloatInRange` -30.0 30.0)) (+ _gravity_point_spawn_loc_z (`KismetMathLibrary.RandomFloatInRange` 20.0 30.0)))) "AdjustIfPossibleButAlwaysSpawn" "OverrideRootScale" null null))
  (set `Actor.Tags` (`|MakeArray` "RoomObjects" :!type "Name") _returnvalue))

(fn `UserConstructionScript`)