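; BP_gravity_objects is a drifting physics cube that reacts to the player's low-poly hand.
; Tick waits a random few seconds, then a timeline blends the cube's velocity toward randomly scaled components of its starting velocity.
; Hand overlap writes a touch event to the first WriteData_BP actor.
; When IsHA is set, finger contact fades the cube from dark grey to red, and ending hand overlap reverses it.
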(event `self.Box.OnComponentBeginOverlap`
  (params (OverlappedComponent :type "PrimitiveComponent Object Reference") (OtherActor :type "Actor Object Reference") (OtherComp :type "PrimitiveComponent Object Reference") (OtherBodyIndex :type Integer) (bFromSweep :type Boolean) (SweepResult :type "HitResult Structure (by ref)"))
  (cast `/UltraleapTracking/InteractionEngine/Pawn/IEUICollisionLowPolyHand` OtherActor)
  (`self.Event` "touch the cube")
  (if (and (`self.isHA`) (`ActorComponent.ComponentHasTag` OtherComp "finger") (not (`self.isTouching?`)))
    (set `self.isTouching?` true)
    (bind (_direction _newtrack_0) (`Timeline|Timeline_1` :!label _label)
      (:`Update`
        (`MeshComponent.SetVectorParameterValueOnMaterials` (`self.Cube`) "color" (`KismetMathLibrary.VLerp` (0.07 0.07 0.07) (1.0 0.0 0.0) _newtrack_0))))))

(event `self.Box.OnComponentEndOverlap`
  (params (OverlappedComponent :type "PrimitiveComponent Object Reference") (OtherActor :type "Actor Object Reference") (OtherComp :type "PrimitiveComponent Object Reference") (OtherBodyIndex :type Integer))
  (cast `/UltraleapTracking/InteractionEngine/Pawn/IEUICollisionLowPolyHand` OtherActor)
  (if (`self.isHA`)
    (set `self.isTouching?` false)
    (goto _label :!via `Reverse`)))

(event `self.ReceiveTick`
  (params (DeltaSeconds :type "Float (single-precision)"))
  (`KismetSystemLibrary.Delay` (`KismetMathLibrary.RandomFloatInRange` 2.0 5.0))
  (bind _returnvalue (`PrimitiveComponent.GetPhysicsLinearVelocity` (`self.Cube`) "None"))
  (bind _output_get (set `self.start_velocity` _returnvalue))
  (bind (_direction _newtrack_0) (`Timeline|Timeline_0`)
    (:`Update`
      (`PrimitiveComponent.SetPhysicsLinearVelocity` (`self.Cube`) (`KismetMathLibrary.VLerp` (`self.start_velocity`) (`KismetMathLibrary.MakeVector` (* (.x _output_get) (`KismetMathLibrary.RandomFloatInRange` -2.0 2.0)) (* (.y _output_get) (`KismetMathLibrary.RandomFloatInRange` -2.0 2.0)) (* (.z _output_get) (`KismetMathLibrary.RandomFloatInRange` -2.0 2.0))) _newtrack_0) false "None"))))

(fn `Event`
  (params (Event :type String))
  (bind _outactors (`GameplayStatics.GetAllActorsOfClass` "/Game/Lisa/WriteData_BP.WriteData_BP_C"))
  (set `/Game/Lisa/WriteData_BP.Event` Event (`|GetArrayItem` _outactors)))

(fn `UserConstructionScript`)