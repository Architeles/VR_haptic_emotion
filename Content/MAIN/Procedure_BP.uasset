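; Procedure controller for an emotion experiment, guiding the participant through a hand-interaction tutorial and arousal/pleasure rooms via Polish banner prompts.
; NextRoom follows the order parsed from ChosenRoomCombination, and SpawnRoom stages each room's cubes, roaches or butterflies.
; A timer clears tagged props and opens an emotion questionnaire.
; Key-routed button presses validate answers, save through WriteData_BP, and insert a gray rest room before advancing.
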(event `Intro`
  (params (`switch on string` :type String))
  (switch `string` `switch on string`
    (:`1`
      (set `self.HeaderText` "INTRO")
      (bind _outactors (`GameplayStatics.GetAllActorsOfClass` "/Game/Lisa/BP_banner.BP_banner_C"))
      (`TextRenderComponent.K2_SetText` (`/Game/Lisa/BP_banner.TextRenderHeading` (`|GetArrayItem` _outactors)) (`self.HeaderText`))
      (`self.set_banner_text` "Witamy w eksperymencie!<br>Trzymaj rece przed soba<br>przez caly czas")
      (`KismetSystemLibrary.Delay` 7.0)
      (`self.set_banner_text` "Zrelaksuj sie i rozejrzyj sie")
      (`KismetSystemLibrary.Delay` 20.0)
      (`self.set_banner_text` "Umiesc reke dokladnie tak,<br> jak jest prezentowana na ekranie<br>(zwroc uwage na to, jak ona jest obrocona)")
      (bind _returnvalue (`|SpawnActorFromClass` "/Game/Lisa/TipHand_BP.TipHand_BP_C" (`KismetMathLibrary.MakeTransform` (`KismetMathLibrary.MakeVector` (`KismetMathLibrary.RandomFloatInRange` -247.0 -203.0) (`KismetMathLibrary.RandomFloatInRange` -410.0 -377.0) (`KismetMathLibrary.RandomFloatInRange` 105.0 115.0)) (`KismetMathLibrary.MakeRotator` 0.0 (`KismetMathLibrary.RandomFloatInRange` -180.0 180.0))) "Undefined" "OverrideRootScale" null null))
      (set `/Game/Lisa/TipHand_BP.room` "Gray" _returnvalue))
    (:`2`
      (`self.set_banner_text` "Dobrze!<br>Przesun zielony punkt na skali<br> blizej odpowiedniego emoji<br>(twoj aktualny stan emocjonalny)")
      (set `self.Key` "QuestTest")
      (bind _asgi_master (cast `/Game/Lisa/GI_Master` (`GameplayStatics.GetGameInstance`)))
      (`|SpawnActorFromClass` "/UltraleapTracking/UIInputModules/InteractableWidgetActor_Master.InteractableWidgetActor_Master_C" (`/Game/Lisa/GI_Master.Questionare_spawn_location` _asgi_master) "Undefined" "OverrideRootScale" null null))
    (:`3`
      (bind _outactors_2 (`GameplayStatics.GetAllActorsOfClass` "/UltraleapTracking/UIInputModules/InteractableWidgetActor_Master.InteractableWidgetActor_Master_C"))
      (`self.K2_DestroyActor` (`|GetArrayItem` _outactors_2))
      (`self.K2_DestroyActor` (`self.ButtonTestIntro`))
      (`self.set_banner_text` "Prawie zaczynamy<br>Zrob 3 glebokie oddechy...")
      (`KismetSystemLibrary.Delay` 10.0)
      (`self.NextRoom`)
      (`KismetSystemLibrary.Delay` 2.0)
      (set `self.HeaderText` "EKSPERYMENT")
      (bind _outactors_3 (`GameplayStatics.GetAllActorsOfClass` "/Game/Lisa/BP_banner.BP_banner_C"))
      (`TextRenderComponent.K2_SetText` (`/Game/Lisa/BP_banner.TextRenderHeading` (`|GetArrayItem` _outactors_3)) (`self.HeaderText`)))))

(event `intro_countinue`
  (`self.set_banner_text` "Sprobuj nacisnac przycisk na stole")
  (bind _asgi_master (cast `/Game/Lisa/GI_Master` (`GameplayStatics.GetGameInstance`)))
  (bind _returnvalue (`|SpawnActorFromClass` "/UltraleapTracking/InteractionEngine/Actors/Button/IEButtonStyledWithText_Master.IEButtonStyledWithText_Master_C" (`/Game/Lisa/GI_Master.Button_spawn_location` _asgi_master) "AlwaysSpawn" "OverrideRootScale" null "/Engine/VREditor/Sounds/UI/Click_on_Button.Click_on_Button" "/Engine/VREditor/Sounds/UI/Click_on_Button.Click_on_Button" true null))
  (bind _output_get (set `self.ButtonTestIntro` _returnvalue))
  (bind _output_get_2 (set `self.button_text` "Nacisnij"))
  (`TextRenderComponent.K2_SetText` (`/UltraleapTracking/InteractionEngine/Actors/Button/IEButtonStyledWithText_Master.TextRender` _output_get) _output_get_2)
  (set `self.Key` "Test"))

(event `self.ReceiveBeginPlay`
  (bind _asgi_master (cast `/Game/Lisa/GI_Master` (`GameplayStatics.GetGameInstance`)))
  (set `self.RoomSpawnLocation` (`/Game/Lisa/GI_Master.Room_spawn_location` _asgi_master)))

(event `self.ReceiveTick`
  (params (DeltaSeconds :type "Float (single-precision)")))

(event `ButtonPressed`
  (switch `string` (`self.Key`)
    (:`Test`
      (`/Engine/EditorBlueprintResources/StandardMacros.DoOnce` false
        (:`Completed`
          (`self.Intro` "2"))))
    (:`QuestTest`
      (bind _outactors (`GameplayStatics.GetAllActorsOfClass` "/UltraleapTracking/UIInputModules/InteractableWidgetActor_Master.InteractableWidgetActor_Master_C"))
      (bind _asbasic_test_umg_master (cast `/UltraleapTracking/UIInputModules/BasicTestUMG_Master` (`WidgetComponent.GetWidget` (`/UltraleapTracking/UIInputModules/InteractableWidgetActor_Master.Widget` (`|GetArrayItem` _outactors)))))
      (if (and (`/UltraleapTracking/UIInputModules/BasicTestUMG_Master.arousal_changed` _asbasic_test_umg_master) (`/UltraleapTracking/UIInputModules/BasicTestUMG_Master.pleasure_changed` _asbasic_test_umg_master))
        (`/Engine/EditorBlueprintResources/StandardMacros.DoOnce` false
          (:`Completed`
            (`self.Intro` "3")
            (bind _outactors_2 (`GameplayStatics.GetAllActorsOfClass` "/Game/Lisa/WriteData_BP.WriteData_BP_C"))
            (`/Game/Lisa/WriteData_BP.SaveDataForm` (`|GetArrayItem` _outactors_2))))
        (else
          (`self.set_banner_text` "Zaznacz swoj stan emocjonalny"))))
    (:`Room`
      (bind _outactors_3 (`GameplayStatics.GetAllActorsOfClass` "/UltraleapTracking/UIInputModules/InteractableWidgetActor_Master.InteractableWidgetActor_Master_C"))
      (bind _asbasic_test_umg_master_2 (cast `/UltraleapTracking/UIInputModules/BasicTestUMG_Master` (`WidgetComponent.GetWidget` (`/UltraleapTracking/UIInputModules/InteractableWidgetActor_Master.Widget` (`|GetArrayItem` _outactors_3)))))
      (if (and (`/UltraleapTracking/UIInputModules/BasicTestUMG_Master.arousal_changed` _asbasic_test_umg_master_2) (`/UltraleapTracking/UIInputModules/BasicTestUMG_Master.pleasure_changed` _asbasic_test_umg_master_2))
        (if (not (`self.close_gate`))
          (set `self.close_gate` true)
          (bind _outactors_4 (`GameplayStatics.GetAllActorsOfClass` "/Game/Lisa/WriteData_BP.WriteData_BP_C"))
          (`/Game/Lisa/WriteData_BP.SaveDataForm` (`|GetArrayItem` _outactors_4))
          (bind _outactors_5 (`GameplayStatics.GetAllActorsWithTag` "ask"))
          (for _array_element _outactors_5
            (`self.K2_DestroyActor` _array_element))
          (bind _outactors_6 (`GameplayStatics.GetAllActorsOfClass` "/Game/Lisa/BP_FadeInAndOut.BP_FadeInAndOut_C"))
          (bind _output (`|GetArrayItem` _outactors_6))
          (`/Game/Lisa/BP_FadeInAndOut.ShowBlack` _output)
          (`KismetSystemLibrary.Delay` 3.0)
          (bind _outactors_7 (`GameplayStatics.GetAllActorsWithTag` "room"))
          (for _array_element_2 _outactors_7
            (`self.K2_DestroyActor` _array_element_2))
          (bind _returnvalue (`|SpawnActorFromClass` "/Game/Lisa/MP_rooms/lisa/mp_rooms/ROOM_gray.ROOM_gray_C" (`KismetMathLibrary.MakeTransform` (`self.RoomSpawnLocation`)) "Undefined" "OverrideRootScale" null null))
          (set `Actor.Tags` (`|MakeArray` "room" :!type "Name") _returnvalue)
          (bind _outactors_8 (`GameplayStatics.GetAllActorsOfClass` "/Game/Lisa/WriteData_BP.WriteData_BP_C"))
          (set `/Game/Lisa/WriteData_BP.Room` "Gray" (`|GetArrayItem` _outactors_8))
          (`/Game/Lisa/BP_FadeInAndOut.RemoveBlack` _output)
          (`self.set_banner_text` "Czas na odpoczynek")
          (`KismetSystemLibrary.Delay` 30.0)
          (`self.NextRoom`)
          (set `self.close_gate` false))
        (else
          (`self.set_banner_text` "Zaznacz swoj stan emocjonalny"))))))

(event `NextRoom`
  (bind _outactors (`GameplayStatics.GetAllActorsOfClass` "/Game/Lisa/BP_FadeInAndOut.BP_FadeInAndOut_C"))
  (bind _output (`|GetArrayItem` _outactors))
  (`/Game/Lisa/BP_FadeInAndOut.ShowBlack` _output)
  (if (== (`KismetArrayLibrary.Array_Length` (`self.Keyboard_rooms`)) 0)
    (`KismetSystemLibrary.PrintString` "END OF THE EXPERIMENT")
    (else
      (`KismetSystemLibrary.Delay` 3.0)
      (bind _output_get (set `self.chosen_Room` (`|GetArrayItem` (`self.RoomCombinationArray_converted`) (`self.Room_index`))))
      (`self.SpawnRoom` _output_get)
      (`KismetArrayLibrary.Array_RemoveItem` (`self.Keyboard_rooms`) (`self.chosen_Room`))
      (`KismetSystemLibrary.Delay` 2.0)
      (`/Game/Lisa/BP_FadeInAndOut.RemoveBlack` _output)
      (`/Engine/EditorBlueprintResources/StandardMacros.IncrementInt` (`self.Room_index`)))))

(event `getRoomCombination`
  (bind _chosenroomcombination (`self.ChosenRoomCombination`))
  (`KismetArrayLibrary.Array_Clear` (`self.RoomCombinationArray`))
  (`KismetArrayLibrary.Array_Clear` (`self.RoomCombinationArray_converted`))
  (`KismetSystemLibrary.PrintString` _chosenroomcombination)
  (for _array_element (`KismetStringLibrary.ParseIntoArray` _chosenroomcombination "," false)
    (`KismetArrayLibrary.Array_Add` (`self.RoomCombinationArray`) _array_element))
  (for _array_element_2 (`self.RoomCombinationArray`)
    (if (`KismetStringLibrary.EqualEqual_StrStr` _array_element_2 "1")
      (`KismetArrayLibrary.Array_Add` (`self.RoomCombinationArray_converted`) "la lp")
      (`KismetSystemLibrary.PrintString` "1")
      (elif (`KismetStringLibrary.EqualEqual_StrStr` _array_element_2 "2")
        (`KismetArrayLibrary.Array_Add` (`self.RoomCombinationArray_converted`) "la hp")
        (`KismetSystemLibrary.PrintString` "2")
        (elif (`KismetStringLibrary.EqualEqual_StrStr` _array_element_2 "3")
          (`KismetArrayLibrary.Array_Add` (`self.RoomCombinationArray_converted`) "ha hp")
          (`KismetSystemLibrary.PrintString` "3")
          (elif (`KismetStringLibrary.EqualEqual_StrStr` _array_element_2 "4")
            (`KismetArrayLibrary.Array_Add` (`self.RoomCombinationArray_converted`) "ha lp")
            (`KismetSystemLibrary.PrintString` "4"))))))
  (for _array_element_3 (`self.RoomCombinationArray_converted`)
    (`KismetSystemLibrary.PrintString` _array_element_3)))

(event `SpawnRoom`
  (params (Room :type String))
  (bind _roomspawnlocation (`self.RoomSpawnLocation`))
  (`KismetSystemLibrary.PrintString` (`VictoryBPFunctionLibrary.AppendMultiple` "spawn room: " Room))
  (bind _outactors (`GameplayStatics.GetAllActorsOfClass` "/Game/Lisa/WriteData_BP.WriteData_BP_C"))
  (set `/Game/Lisa/WriteData_BP.Room` Room (`|GetArrayItem` _outactors))
  (bind _returnvalue (`KismetSystemLibrary.K2_SetTimer` null "CleanTheRoom" (`self.Room_time`)))
  (set `self.Timer` _returnvalue)
  (switch `string` Room
    (:`la lp`
      ;[1 1 1] LA LP 1
      (bind _outactors_2 (`GameplayStatics.GetAllActorsWithTag` "room"))
      (for _array_element _outactors_2
        (`self.K2_DestroyActor` _array_element))
      (bind _returnvalue_2 (`|SpawnActorFromClass` "/Game/Lisa/MP_rooms/lisa/mp_rooms/ROOM_la_nv.ROOM_la_nv_C" (`KismetMathLibrary.MakeTransform` _roomspawnlocation) "Undefined" "OverrideRootScale" null null))
      (set `Actor.Tags` (`|MakeArray` "room" :!type "Name") _returnvalue_2)
      (bind _outactors_3 (`GameplayStatics.GetAllActorsOfClass` "/Game/Lisa/WriteData_BP.WriteData_BP_C"))
      (set `/Game/Lisa/WriteData_BP.Room` "la lp" (`|GetArrayItem` _outactors_3))
      (`self.set_banner_text` "Rozejrzyj sie")
      (`self.Event` "adaptation to the room")
      (`KismetSystemLibrary.Delay` (`self.Adaption_time`))
      (`self.Spawn Gravity` false)
      (`self.set_banner_text` "Zlap kostki!")
      (`self.Event` "cubes spawned")
      (set `self.Key` "Room"))
    (:`la hp`
      ;[1 1 1] LA HP 2
      (bind _outactors_4 (`GameplayStatics.GetAllActorsWithTag` "room"))
      (for _array_element_2 _outactors_4
        (`self.K2_DestroyActor` _array_element_2))
      (bind _returnvalue_3 (`|SpawnActorFromClass` "/Game/Lisa/MP_rooms/lisa/mp_rooms/ROOM_la_pv.ROOM_la_pv_C" (`KismetMathLibrary.MakeTransform` _roomspawnlocation) "Undefined" "OverrideRootScale" null null))
      (set `Actor.Tags` (`|MakeArray` "room" :!type "Name") _returnvalue_3)
      (bind _outactors_5 (`GameplayStatics.GetAllActorsOfClass` "/Game/Lisa/WriteData_BP.WriteData_BP_C"))
      (set `/Game/Lisa/WriteData_BP.Room` "la hp" (`|GetArrayItem` _outactors_5))
      (`self.set_banner_text` "Rozejrzyj sie")
      (`self.Event` "adaptation to the room")
      (`KismetSystemLibrary.Delay` (`self.Adaption_time`))
      (`self.Spawn Gravity` true)
      (`self.Event` "cubes spawned")
      (`self.set_banner_text` "Dotknij kostki!")
      (set `self.Key` "Room"))
    (:`ha lp`
      ;[1 1 1] HA LP 4
      (bind _outactors_6 (`GameplayStatics.GetAllActorsWithTag` "room"))
      (for _array_element_3 _outactors_6
        (`self.K2_DestroyActor` _array_element_3))
      (bind _returnvalue_4 (`|SpawnActorFromClass` "/Game/Lisa/MP_rooms/lisa/mp_rooms/ROOM_ha_np.ROOM_ha_np_C" (`KismetMathLibrary.MakeTransform` _roomspawnlocation) "Undefined" "OverrideRootScale" null null))
      (set `Actor.Tags` (`|MakeArray` "room" :!type "Name") _returnvalue_4)
      (bind _outactors_7 (`GameplayStatics.GetAllActorsOfClass` "/Game/Lisa/WriteData_BP.WriteData_BP_C"))
      (set `/Game/Lisa/WriteData_BP.Room` "ha lp" (`|GetArrayItem` _outactors_7))
      (`self.set_banner_text` "Rozejrzyj sie")
      (`self.Event` "adaptation to the room")
      (for _ (range 11)
        (bind _returnvalue_5 (`|SpawnActorFromClass` "/Game/Lisa/Roach_Mob.Roach_Mob_C" (`KismetMathLibrary.MakeTransform` (`KismetMathLibrary.MakeVector` (`KismetMathLibrary.RandomFloatInRange` -83.0 -284.0) (`KismetMathLibrary.RandomFloatInRange` -114.0 -578.0) 9.0) (`KismetMathLibrary.MakeRotator` 0.0 0.0 (`KismetMathLibrary.RandomFloatInRange` 0.0 360.0))) "AdjustIfPossibleButAlwaysSpawn" "OverrideRootScale" null null))
        (set `Actor.Tags` (`self.RoomObjects`) _returnvalue_5))
      (`KismetSystemLibrary.Delay` (`self.Adaption_time`))
      (`/Game/Lisa/MyMacroLib.ForLoopWithDelay` 0 4 0.2 2.0
        (:`LoopBody`
          (bind _returnvalue_6 (`|SpawnActorFromClass` "/Game/Lisa/Roach_Mob_blessed.Roach_Mob_blessed_C" (`KismetMathLibrary.MakeTransform` (`KismetMathLibrary.MakeVector` (`KismetMathLibrary.RandomFloatInRange` -254.0 -158.0) (`KismetMathLibrary.RandomFloatInRange` -388.0 -346.0) 300.0) (`KismetMathLibrary.MakeRotator` 0.0 0.0 (`KismetMathLibrary.RandomFloatInRange` 0.0 360.0))) "AdjustIfPossibleButAlwaysSpawn" "OverrideRootScale" null null))
          (set `Actor.Tags` (`self.RoomObjects`) _returnvalue_6))
        (:`Complited`
          (`self.set_banner_text` "Dotknij karalucha")
          (`self.Event` "roaches spawned")
          (`KismetSystemLibrary.Delay` 35.0)
          (bind _asgi_master (cast `/Game/Lisa/GI_Master` (`GameplayStatics.GetGameInstance`)))
          (bind _returnvalue_7 (`|SpawnActorFromClass` "/Game/Lisa/TipHand_BP.TipHand_BP_C" (`KismetMathLibrary.MakeTransform` (`/Game/Lisa/GI_Master.TipHand_loc` _asgi_master)) "Undefined" "OverrideRootScale" null null))
          (set `Actor.Tags` (`self.RoomObjects`) _returnvalue_7)
          (set `/Game/Lisa/TipHand_BP.room` "ha lp" _returnvalue_7)
          (set `/Game/Lisa/TipHand_BP.timeToJump` true _returnvalue_7)
          (`self.set_banner_text` "Teraz spojrz w prawo i umiesc<br>prawa otwarta dlon w pozycji<br> wyswietlanej na ekranie")
          (`self.Event` "wait for a hand")
          (set `self.Key` "Room"))))
    (:`ha hp`
      ;[1 1 1] HA HP 3
      (bind _outactors_8 (`GameplayStatics.GetAllActorsWithTag` "room"))
      (for _array_element_4 _outactors_8
        (`self.K2_DestroyActor` _array_element_4))
      (bind _returnvalue_8 (`|SpawnActorFromClass` "/Game/Lisa/MP_rooms/lisa/mp_rooms/ROOM_ha_pv.ROOM_ha_pv_C" (`KismetMathLibrary.MakeTransform` _roomspawnlocation) "Undefined" "OverrideRootScale" null null))
      (set `Actor.Tags` (`|MakeArray` "room" :!type "Name") _returnvalue_8)
      (bind _outactors_9 (`GameplayStatics.GetAllActorsOfClass` "/Game/Lisa/WriteData_BP.WriteData_BP_C"))
      (set `/Game/Lisa/WriteData_BP.Room` "ha hp" (`|GetArrayItem` _outactors_9))
      (`self.set_banner_text` "Rozejrzyj sie")
      (`self.Event` "adaptation to the room")
      (`KismetSystemLibrary.Delay` (`self.Adaption_time`))
      (`/Game/Lisa/MyMacroLib.ForLoopWithDelay` 0 3
        (:`LoopBody`
          (bind _returnvalue_9 (`|SpawnActorFromClass` "/Game/Lisa/moth/Butterfly_BP.Butterfly_BP_C" (`KismetMathLibrary.MakeTransform` (`KismetMathLibrary.MakeVector` (`KismetMathLibrary.RandomFloatInRange` -74.0 -122.0) (`KismetMathLibrary.RandomFloatInRange` -44.0 82.0) (`KismetMathLibrary.RandomFloatInRange` 44.0 213.0)) (`KismetMathLibrary.MakeRotator` 0.0 0.0 (`KismetMathLibrary.RandomFloatInRange` 0.0 360.0))) "Undefined" "OverrideRootScale" null null))
          (set `Actor.Tags` (`self.RoomObjects`) _returnvalue_9))
        (:`Complited`
          (`self.Event` "butterfly spawned")
          (`KismetSystemLibrary.Delay` 30.0)
          (`self.set_banner_text` "Umiesc prawa dlon w miejsce wskazane<br>na ekranie, obroc dlon w dol")
          (bind _returnvalue_10 (`|SpawnActorFromClass` "/Game/Lisa/TipHand_BP.TipHand_BP_C" (`KismetMathLibrary.MakeTransform` (`KismetMathLibrary.MakeVector` -210.454666 -379.70285 110.26738) (struct :`Yaw` 180.0 :`Roll` -180.0)) "Undefined" "OverrideRootScale" null null))
          (set `Actor.Tags` (`self.RoomObjects`) _returnvalue_10)
          (set `/Game/Lisa/TipHand_BP.room` "ha hp" _returnvalue_10)
          (set `self.Key` "Room"))))
    (:`Gray`
      ;[1 1 1] GRAY
      (bind _outactors_10 (`GameplayStatics.GetAllActorsWithTag` "room"))
      (for _array_element_5 _outactors_10
        (`self.K2_DestroyActor` _array_element_5))
      (bind _returnvalue_11 (`|SpawnActorFromClass` "/Game/Lisa/MP_rooms/lisa/mp_rooms/ROOM_gray.ROOM_gray_C" (`KismetMathLibrary.MakeTransform` _roomspawnlocation) "Undefined" "OverrideRootScale" null null))
      (set `Actor.Tags` (`|MakeArray` "room" :!type "Name") _returnvalue_11)
      (bind _outactors_11 (`GameplayStatics.GetAllActorsOfClass` "/Game/Lisa/WriteData_BP.WriteData_BP_C"))
      (set `/Game/Lisa/WriteData_BP.Room` "Gray" (`|GetArrayItem` _outactors_11)))))

(fn `ask_opinion`
  (`self.set_banner_text` "Przesun zielony punkt na skali<br> blizej odpowiedniego emoji<br>(twoj aktualny stan emocjonalny)")
  (bind _asgi_master (cast `/Game/Lisa/GI_Master` (`GameplayStatics.GetGameInstance`)))
  (bind _returnvalue (`|SpawnActorFromClass` "/UltraleapTracking/InteractionEngine/Actors/Button/IEButtonStyledWithText_Master.IEButtonStyledWithText_Master_C" (`/Game/Lisa/GI_Master.Button_spawn_location` _asgi_master) "AlwaysSpawn" "OverrideRootScale" null "/Engine/VREditor/Sounds/UI/Click_on_Button.Click_on_Button" "/Engine/VREditor/Sounds/UI/Click_on_Button.Click_on_Button" true null))
  (set `Actor.Tags` (`|MakeArray` "ask" :!type "Name") _returnvalue)
  (bind _asgi_master_2 (cast `/Game/Lisa/GI_Master` (`GameplayStatics.GetGameInstance`)))
  (bind _returnvalue_2 (`|SpawnActorFromClass` "/UltraleapTracking/UIInputModules/InteractableWidgetActor_Master.InteractableWidgetActor_Master_C" (`/Game/Lisa/GI_Master.Questionare_spawn_location` _asgi_master_2) "Undefined" "OverrideRootScale" null null))
  (set `Actor.Tags` (`|MakeArray` "ask" :!type "Name") _returnvalue_2))

(fn `CleanTheRoom`
  (bind _outactors (`GameplayStatics.GetAllActorsWithTag` "RoomObjects"))
  (for _array_element _outactors
    (`self.K2_DestroyActor` _array_element))
  (`self.ask_opinion`))

(fn `Event`
  (params (`Event to send` :type String))
  (bind _outactors (`GameplayStatics.GetAllActorsOfClass` "/Game/Lisa/WriteData_BP.WriteData_BP_C"))
  (set `/Game/Lisa/WriteData_BP.Event` `Event to send` (`|GetArrayItem` _outactors)))

(fn `set_banner_text`
  (params (Text :type Text))
  (bind _outactors (`GameplayStatics.GetAllActorsOfClass` "/Game/Lisa/BP_banner.BP_banner_C"))
  (`TextRenderComponent.K2_SetText` (`/Game/Lisa/BP_banner.TextRender` (`|GetArrayItem` _outactors)) Text)
  (`GameplayStatics.PlaySoundAtLocation` "/UltraleapTracking/InteractionEngine/Keyboard/Sounds/glass_006_Cue.glass_006_Cue" (0.0 0.0 0.0) (struct) 1.0 1.0 0.0 null null null))

(fn `Spawn Gravity`
  (params (`is_la_hp?` :type Boolean))
  (bind _asgi_master (cast `/Game/Lisa/GI_Master` (`GameplayStatics.GetGameInstance`)))
  (bind _returnvalue (`|SpawnActorFromClass` "/Game/Lisa/Particles/BP_gravity/BP_gravity.BP_gravity_C" (`KismetMathLibrary.MakeTransform` (`/Game/Lisa/GI_Master.Gravity_point_spawn_loc` _asgi_master)) "Undefined" "OverrideRootScale" null null))
  (set `Actor.Tags` (`self.RoomObjects`) _returnvalue)
  (set `/Game/Lisa/Particles/BP_gravity/BP_gravity.is_la_hp?` `is_la_hp?` _returnvalue)
  (for _ (range 9)
    (bind (_gravity_point_spawn_loc_x _gravity_point_spawn_loc_y _gravity_point_spawn_loc_z) (`KismetMathLibrary.BreakVector` (`/Game/Lisa/GI_Master.Gravity_point_spawn_loc` _asgi_master)))
    (bind _returnvalue_2 (`|SpawnActorFromClass` "/Game/Lisa/Particles/BP_gravity/BP_gravity_objects.BP_gravity_objects_C" (`KismetMathLibrary.MakeTransform` (`KismetMathLibrary.MakeVector` (+ _gravity_point_spawn_loc_x (`KismetMathLibrary.RandomFloatInRange` -60.0 60.0)) (+ _gravity_point_spawn_loc_y (`KismetMathLibrary.RandomFloatInRange` -60.0 60.0)) (+ _gravity_point_spawn_loc_z (`KismetMathLibrary.RandomFloatInRange` 20.0 60.0)))) "AdjustIfPossibleButAlwaysSpawn" "OverrideRootScale" null null))
    (set `Actor.Tags` (`self.RoomObjects`) _returnvalue_2)))

(fn `UserConstructionScript`)