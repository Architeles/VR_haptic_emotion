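; TipHand_BP is a hand-target actor that reacts to the player's low-poly hand according to the Room name.
; Capsule overlap with the right hand pauses the butterfly's random flight in "ha hp"; elsewhere, when TimeToJump, it toggles the roach's jump to hand.
; Tick respawns a fallen roach at "roach_birth" and re-triggers finished jumps.
; In "Gray", Sphere touches relocate it randomly until a count continues Procedure_BP's intro and destroys it.
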(event `self.ReceiveBeginPlay`
  (`KismetSystemLibrary.Delay` 1.0)
  (if (`KismetStringLibrary.EqualEqual_StrStr` (`self.room`) "ha hp")
    (bind _outactors (`GameplayStatics.GetAllActorsOfClass` "/Game/Lisa/moth/Butterfly_BP.Butterfly_BP_C"))
    (bind _output_get (set `self.Butterfly` (`|GetArrayItem` _outactors)))
    (`SceneComponent.SetHiddenInGame` (`/Game/Lisa/moth/Butterfly_BP.Arrow` _output_get) true false)
    (else
      (bind _outactors_2 (`GameplayStatics.GetAllActorsOfClass` "/Game/Lisa/Roach_Mob_blessed.Roach_Mob_blessed_C"))
      (bind _output (`|GetArrayItem` _outactors_2))
      (`/Engine/EditorBlueprintResources/StandardMacros.IsValid` _output
        (:`Is Valid`
          (set `self.Roach` _output))))))

(event `self.ReceiveTick`
  (params (DeltaSeconds :type "Float (single-precision)"))
  (bind _roach (`self.Roach`))
  (bind (_returnvalue_x _returnvalue_y _returnvalue_z) (`KismetMathLibrary.BreakVector` (`self.K2_GetActorLocation` (`self.Roach`))))
  (bind _jumpdone (`/Game/Lisa/Roach_Mob_blessed.jumpDone` _roach))
  (bind _jumptohand_ (`/Game/Lisa/Roach_Mob_blessed.JumpToHand?` _roach))
  (if (not (`KismetStringLibrary.EqualEqual_StrStr` (`self.room`) "ha hp"))
    (`/Engine/EditorBlueprintResources/StandardMacros.IsValid` (`self.Roach`)
      (:`Is Valid`
        (if (< _returnvalue_z 40.0)
          (bind _outactors (`GameplayStatics.GetAllActorsWithTag` "roach_birth"))
          (`self.K2_SetActorLocation` (`self.Roach`) (`self.K2_GetActorLocation` (`|GetArrayItem` _outactors)) false false)
          (elif (`self.timeToJump`)
            (for _array_element (`PrimitiveComponent.GetOverlappingActors` (`self.Capsule`) null)
              (if (`.bSuccess` (cast `/UltraleapTracking/InteractionEngine/Pawn/IEUICollisionLowPolyHand` _array_element :!pure true))
                (`KismetSystemLibrary.PrintString` (`VictoryBPFunctionLibrary.AppendMultiple` "Jump done?    " (`KismetStringLibrary.Conv_BoolToString` _jumpdone)))
                (if _jumpdone
                  (`KismetSystemLibrary.PrintString` (`VictoryBPFunctionLibrary.AppendMultiple` "Jump to hand?    " (`KismetStringLibrary.Conv_BoolToString` _jumptohand_)))
                  (set `/Game/Lisa/Roach_Mob_blessed.jumpDone` false _roach)
                  (set `/Game/Lisa/Roach_Mob_blessed.JumpToHand?` true _roach)
                  (else
                    (`KismetSystemLibrary.PrintString` (`KismetStringLibrary.Concat_StrStr` "Jump doesnt done. Jump to hand?      " (`KismetStringLibrary.Conv_BoolToString` _jumptohand_)))))))))))))

(event `self.Capsule.OnComponentBeginOverlap`
  (params (OverlappedComponent :type "PrimitiveComponent Object Reference") (OtherActor :type "Actor Object Reference") (OtherComp :type "PrimitiveComponent Object Reference") (OtherBodyIndex :type Integer) (bFromSweep :type Boolean) (SweepResult :type "HitResult Structure (by ref)"))
  (bind _asieuicollision_low_poly_hand (cast `/UltraleapTracking/InteractionEngine/Pawn/IEUICollisionLowPolyHand` OtherActor))
  (if (== (`/UltraleapTracking/BodyState/BSLowPolyHand.Right` _asieuicollision_low_poly_hand) OtherComp)
    (if (`KismetStringLibrary.EqualEqual_StrStr` (`self.room`) "ha hp")
      (set `/Game/Lisa/moth/Butterfly_BP.RandomFlying` false (`self.Butterfly`))
      (elif (`self.timeToJump`)
        (`SceneComponent.SetHiddenInGame` (`/Game/Lisa/Roach_Mob_blessed.Arrow1` (`self.Roach`)) true false)
        (set `/Game/Lisa/Roach_Mob_blessed.JumpToHand?` true (`self.Roach`))))))

(event `self.Capsule.OnComponentEndOverlap`
  (params (OverlappedComponent :type "PrimitiveComponent Object Reference") (OtherActor :type "Actor Object Reference") (OtherComp :type "PrimitiveComponent Object Reference") (OtherBodyIndex :type Integer))
  (bind _asieuicollision_low_poly_hand (cast `/UltraleapTracking/InteractionEngine/Pawn/IEUICollisionLowPolyHand` OtherActor))
  (if (== (`/UltraleapTracking/BodyState/BSLowPolyHand.Right` _asieuicollision_low_poly_hand) OtherComp)
    (if (`KismetStringLibrary.EqualEqual_StrStr` (`self.room`) "ha hp")
      (set `/Game/Lisa/moth/Butterfly_BP.RandomFlying` true (`self.Butterfly`))
      (elif (`self.timeToJump`)
        (`SceneComponent.SetHiddenInGame` (`/Game/Lisa/Roach_Mob_blessed.Arrow1` (`self.Roach`)) true false)
        (set `/Game/Lisa/Roach_Mob_blessed.JumpToHand?` false (`self.Roach`))))))

(event `self.Sphere.OnComponentBeginOverlap`
  (params (OverlappedComponent :type "PrimitiveComponent Object Reference") (OtherActor :type "Actor Object Reference") (OtherComp :type "PrimitiveComponent Object Reference") (OtherBodyIndex :type Integer) (bFromSweep :type Boolean) (SweepResult :type "HitResult Structure (by ref)"))
  (if (`KismetStringLibrary.EqualEqual_StrStr` (`self.room`) "Gray")
    (if (>= (`self.counter`) 5)
      (bind _outactors (`GameplayStatics.GetAllActorsOfClass` "/Game/Lisa/Procedure_BP.Procedure_BP_C"))
      (`/Game/Lisa/Procedure_BP.intro_countinue` (`|GetArrayItem` _outactors))
      (`self.K2_DestroyActor`)
      (else
        (bind _asieuicollision_low_poly_hand (cast `/UltraleapTracking/InteractionEngine/Pawn/IEUICollisionLowPolyHand` OtherActor))
        (if (== (`/UltraleapTracking/BodyState/BSLowPolyHand.Right` _asieuicollision_low_poly_hand) OtherComp)
          (`KismetSystemLibrary.Delay` 2.0)
          (`self.K2_SetActorLocationAndRotation` (`KismetMathLibrary.MakeVector` (`KismetMathLibrary.RandomFloatInRange` -225.0 -203.0) (`KismetMathLibrary.RandomFloatInRange` -410.0 -387.0) (`KismetMathLibrary.RandomFloatInRange` 105.0 115.0)) (`KismetMathLibrary.MakeRotator` 0.0 (`KismetMathLibrary.RandomFloatInRange` -180.0 180.0)))
          (`/Engine/EditorBlueprintResources/StandardMacros.IncrementInt` (`self.counter`)))))))

(fn `UserConstructionScript`)