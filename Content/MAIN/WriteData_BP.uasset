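; WriteData_BP logs participant data, apparently for a haptics experiment, to timestamp-named text files in the project directory.
; createFiles writes headers for a form file (arousal, pleasure, haptic flag, demographics) and a procedure file; two save events append rows to them.
; Tick refreshes the clock string and copies touch state from the BP_SerialComv3_UE427 serial actor.
; Hand-overlap logic for naming touched actors exists but is disconnected, so it never runs.
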(event `self.ReceiveBeginPlay`
  (bind _outactors (`GameplayStatics.GetAllActorsOfClass` "/Game/Lisa/BP_SerialCom-v3_UE427.BP_SerialCom-v3_UE427_C"))
  (set `self.serial_port` (`|GetArrayItem` _outactors)))

(event `createFiles`
  (bind _returnvalue (`KismetSystemLibrary.GetProjectDirectory`))
  (bind (_returnvalue_year _returnvalue_month _returnvalue_day _returnvalue_hour _returnvalue_minute _returnvalue_second) (`KismetMathLibrary.BreakDateTime` (`KismetMathLibrary.Now`)))
  (bind _output_get (set `self.File_name` (`KismetStringLibrary.Concat_StrStr` (`KismetStringLibrary.Conv_IntToString` _returnvalue_day) "-" (`KismetStringLibrary.Conv_IntToString` _returnvalue_month) " " (`KismetStringLibrary.Conv_IntToString` _returnvalue_hour) "-" (`KismetStringLibrary.Conv_IntToString` _returnvalue_minute) "-" (`KismetStringLibrary.Conv_IntToString` _returnvalue_second) ".txt")))
  (`VictoryBPFunctionLibrary.FileIO__SaveStringTextToFile` _returnvalue _output_get (`KismetStringLibrary.Concat_StrStr` "Time" " " "Room" " " "Arousal" " " "Pleasure" " " "isHaptyc" " " "Sex" " " "Age") true true)
  (`VictoryBPFunctionLibrary.FileIO__SaveStringTextToFile` _returnvalue (`VictoryBPFunctionLibrary.AppendMultiple` "Procedure " (`self.File_name`)) (`KismetStringLibrary.Concat_StrStr` "Time" " " "Room" " " "isTouching?" " " "Event") true true)
  (set `self.ready` true)
  (bind _outactors (`GameplayStatics.GetAllActorsOfClass` "/UltraleapTracking/InteractionEngine/Pawn/IEUICollisionLowPolyHand.IEUICollisionLowPolyHand_C"))
  (set `self.HandRef` (`|GetArrayItem` _outactors)))

(event `SaveDataForm`
  (`VictoryBPFunctionLibrary.FileIO__SaveStringTextToFile` (`KismetSystemLibrary.GetProjectDirectory`) (`self.File_name`) (`KismetStringLibrary.Concat_StrStr` (`self.Time`) " " (`self.Room`) " " (`self.Arousal`) " " (`self.Pleasure`) " " (`self.isHaptyc`) " " (`self.sex`) " " (`self.age`)) true true))

(event `SaveProcedureData`
  (`VictoryBPFunctionLibrary.FileIO__SaveStringTextToFile` (`KismetSystemLibrary.GetProjectDirectory`) (`VictoryBPFunctionLibrary.AppendMultiple` "Procedure " (`self.File_name`)) (`KismetStringLibrary.Concat_StrStr` (`self.Time`) " " (`self.Room`) " " (`self.isTouching?`) " " (`self.Event`)) true true))

(event `self.ReceiveTick`
  (params (DeltaSeconds :type "Float (single-precision)"))
  (bind (_returnvalue_year _returnvalue_month _returnvalue_day _returnvalue_hour _returnvalue_minute _returnvalue_second _returnvalue_millisecond) (`KismetMathLibrary.BreakDateTime` (`KismetMathLibrary.Now`)))
  (set `self.isTouching?` (`/Game/Lisa/BP_SerialCom-v3_UE427.isTouching` (`self.serial_port`)))
  (set `self.Time` (`KismetStringLibrary.Concat_StrStr` (`KismetStringLibrary.Conv_IntToString` _returnvalue_hour) ":" (`KismetStringLibrary.Conv_IntToString` _returnvalue_minute) ":" (`KismetStringLibrary.Conv_IntToString` _returnvalue_second)))
  (if (`self.ready`)
    _))

(fn `UserConstructionScript`)