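; BP_FadeInAndOut fades the scene in from black and back out through the color Gain of its PostProcess component.
; On BeginPlay it sets Gain to black, waits briefly, then calls RemoveBlack.
; RemoveBlack plays a timeline whose alpha drives all four Gain channels, and ShowBlack reverses the same timeline to return to black.
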(event `self.ReceiveBeginPlay`
  ;[1 1 1] Make Scene PP Black As Default
  (setmembers `PostProcessSettings` :`StructRef` (`PostProcessVolume.Settings` (`self.PostProcess`)) :`ColorGain` (`KismetMathLibrary.MakeVector4` 0.0))
  (`KismetSystemLibrary.Delay` 2.0)
  (`self.RemoveBlack`))

(event `RemoveBlack`
  ;[1 1 1] Show Or Hide Scene PP
  (bind (_direction _alpha1) (`Timeline|Timeline_0` :!label _label)
    (:`Update`
      (setmembers `PostProcessSettings` :`StructRef` (`PostProcessVolume.Settings` (`self.PostProcess`)) :`ColorGain` (`KismetMathLibrary.MakeVector4` _alpha1 _alpha1 _alpha1 _alpha1)))))

(event `ShowBlack`
  ;[1 1 1] Show Or Hide Scene PP
  (goto _label :!via `Reverse`))

(fn `UserConstructionScript`)